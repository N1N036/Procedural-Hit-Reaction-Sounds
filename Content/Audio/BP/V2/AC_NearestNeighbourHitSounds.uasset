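; Actor component that plays velocity-matched impact sounds from a sliced wave asset when its owner is hit.
; AnalyseOnsets, not called at runtime here, maps onset strengths to timestamps and builds a nearest-neighbour lookup table by velocity.
; Hits move a spawned AmbientSound, index that table by scaled speed and set MetaSound start and decay times.
; A randomised cooldown throttles hits; results matching LastSamplePosResult shift to an adjacent onset.
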(event Custom|OnActorhit
  (params (SelfActor :type Actor%20Object%20Reference) (OtherActor :type Actor%20Object%20Reference) (NormalImpulse :type Vector) (Hit :type Hit%20Result%20Structure%20%28by%20ref%29))
  (CallFunction|TriggerHitSounds (Transformation|GetVelocity (Components|GetOwner)) (Transformation|GetActorTransform SelfActor)))

(event Custom|TriggerHitSounds
  (params (Velocity :type Vector) (NewTransform :type Transform%20%28by%20ref%29))
  (bind _returnvalue (Math|Vector|VectorLength Velocity))
  (bind _nearestneighbourresults (Variables|Default|GetNearestNeighbourResults))
  (bind _audiocomp (Variables|Default|GetAudioComp))
  (bind _audiocomponent (Variables|/Script/Engine.AmbientSound|GetAudioComponent _audiocomp))
  (Utilities|FlowControl|Sequence
    (:then_0
      (Utilities|FlowControl|DoOnce false :!label _label
        (:Completed
          (if (> _returnvalue 0.1)
            (Variables|Default|SetScaledVelocity (/ _returnvalue 1e+03))
            (Transformation|SetWorldTransform _audiocomponent NewTransform false true)
            (Audio|Components|Audio|Play _audiocomponent 0.0)
            (Class|AudioComponent|SetWaveParameter _audiocomponent "WaveAsset" (Variables|Default|GetWaveAsset))
            (Utilities|FlowControl|Sequence
              (:then_0
                (if (Utilities|Array|IsValidIndex _nearestneighbourresults (Math|Float|Truncate (* (Variables|Default|GetScaledVelocity) 1e+02)))
                  (if (== (Utilities|Array|Get(acopy) _nearestneighbourresults (Math|Float|Truncate (* (Variables|Default|GetScaledVelocity) 1e+02))) (Variables|Default|GetLastSamplePosResult))
                    (bind _values (Utilities|Map|Values (Variables|Default|GetOnsetTimestampMap)))
                    (Variables|Default|SetSamplePosResult (Utilities|Array|Get(acopy) _values (+ (Utilities|Array|FindItem _values (stale _output_get)) (Math|Integer|SelectInt 1 -1 (Math|Random|RandomBool)))))
                    (else
                      (bind _output_get (Variables|Default|SetSamplePosResult (Utilities|Array|Get(acopy) _nearestneighbourresults (Math|Float|Truncate (* (Variables|Default|GetScaledVelocity) 1e+02)))))))))
              (:then_1
                (Audio|Parameter|SetFloatParameter _audiocomponent "StartTime" (Variables|Default|GetSamplePosResult) :!class /Script/AudioExtensions.AudioParameterControllerInterface)
                (Audio|Parameter|SetFloatParameter _audiocomponent "DecayTime" (Variables|Default|GetScaledVelocity) :!class /Script/AudioExtensions.AudioParameterControllerInterface)))))))
    (:then_1
      (Utilities|FlowControl|Delay (Math|Random|RandomFloatinRange 0.5 1.0))
      (goto _label Reset))))

(event EventBeginPlay
  (bind _returnvalue (Components|GetOwner))
  (Variables|Default|SetIsInitialized true)
  (if (Utilities|IsValid _returnvalue)
    (Collision|BindEventtoOnActorHit _returnvalue (delegate Custom|OnActorhit))
    (bind _returnvalue_2 (Game|SpawnActorfromClass "/Script/Engine.AmbientSound" (Transformation|GetActorTransform _returnvalue) "Undefined" _returnvalue 0))
    (bind _output_get (Variables|Default|SetAudioComp _returnvalue_2))
    (Audio|Components|Audio|SetSound (Variables|/Script/Engine.AmbientSound|GetAudioComponent _output_get) (Variables|Default|GetMSS%20Transient%20Select))
    (Variables|/Script/Engine.AudioComponent|SetAttenuationSettings (Variables|/Script/Engine.AmbientSound|GetAudioComponent _output_get) (Variables|Default|GetAttenuation))))

(event EventTick
  (params (DeltaSeconds :type Float%20%28single-precision%29)))

(fn AnalyseOnsets
  (bind _onsetnrt (Variables|Default|GetOnsetNRT))
  (bind _durationinseconds (Variables|/Script/AudioAnalyzer.AudioAnalyzerNRT|GetDurationInSeconds _onsetnrt))
  (bind (_outonsettimestamps _outonsetstrengths) (Class|OnsetNRT|GetNormalizedChannelOnsetsBetweenTimes _onsetnrt 0.0 _durationinseconds))
  ;[1 1 1] OnsetDatamap(floats)
  (for (_array_element _array_index) _outonsettimestamps
    (Utilities|Map|Add (Variables|Default|GetOnsetTimestampMap) (Utilities|Array|Get(acopy) _outonsetstrengths _array_index) _array_element))
  (for _index (range 0 100)
    (bind _output (CallFunction|NearestNeighbourAnalysis (Math|Float|SafeDivide (Math|Conversions|ToFloat(Integer) _index) 1e+02)))
    (Utilities|Array|SetArrayElem (Variables|Default|GetNearestNeighbourResults) _index _output true)))

(fn NearestNeighbourAnalysis
  (params (ScaledVelocity :type Float%20%28double-precision%29))
  (bind _sorteddiffarray (Variables|Default|GetSortedDiffArray))
  (bind _onsettimestampmap (Variables|Default|GetOnsetTimestampMap))
  (bind _indexofminvalue (Math|Float|MinOfFloatArray _sorteddiffarray))
  (Variables|Default|SetScaledVelocity ScaledVelocity)
  (bind _keys (Utilities|Map|Keys _onsettimestampmap))
  (for (_array_element _array_index) _keys
    (Utilities|Array|SetArrayElem _sorteddiffarray _array_index (Math|Float|Absolute(Float) (- (Variables|Default|GetScaledVelocity) _array_element)) true)
    (bind _values (Utilities|Map|Values _onsettimestampmap)))
  (if (Utilities|Array|IsValidIndex _values _indexofminvalue)
    (return (Utilities|Array|Get(acopy) _values _indexofminvalue))))