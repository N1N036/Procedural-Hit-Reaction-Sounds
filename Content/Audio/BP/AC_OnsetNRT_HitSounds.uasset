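; Actor component that plays velocity-matched impact sounds from one wave asset when its owner is hit.
; On init it spawns an AmbientSound running a MetaSound and loads precomputed onset-analysis data for SoundName from an EUA_UpdateNRT actor.
; Hit speed indexes nearest-neighbour onset times to set the MetaSound's start time, stepping to a neighbouring onset on repeats.
; Sound moves to the hit location, throttled by speed, play-state and random-delay gates.
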(event Custom|OnActorhit
  (params (SelfActor :type Actor%20Object%20Reference) (OtherActor :type Actor%20Object%20Reference) (NormalImpulse :type Vector) (Hit :type Hit%20Result%20Structure%20%28by%20ref%29))
  (bind _audiocomponent (Variables|Default|GetAudioComponent))
  (bind _nearestneighbourresults (Variables|Default|GetNearestNeighbourResults))
  (bind _owner (Variables|Default|GetOwner))
  (bind _returnvalue (Transformation|GetVelocity _owner))
  (bind _returnvalue_2 (Math|Vector|VectorLength _returnvalue))
  (Utilities|FlowControl|Sequence
    (:then_0
      (Utilities|FlowControl|DoOnce false :!label _label
        (:Completed
          (if (not (Audio|Components|Audio|IsPlaying (Audio|Components|Audio|GetPlayState (Variables|Default|GetAudioComponent))))
            (if (> _returnvalue_2 2e+01)
              (Variables|Default|SetScaledVelocity (/ _returnvalue_2 1e+03))
              (Transformation|SetWorldTransform _audiocomponent (Math|Conversions|ToTransform(Vector) (.location Hit)) false true)
              (Audio|Components|Audio|Play _audiocomponent 0.0)
              (Utilities|FlowControl|Sequence
                (:then_0
                  (if (Utilities|Array|IsValidIndex _nearestneighbourresults (Math|Float|Truncate (* (Variables|Default|GetScaledVelocity) 1e+02)))
                    (if (== (Utilities|Array|Get(acopy) _nearestneighbourresults (Math|Float|Truncate (* (Variables|Default|GetScaledVelocity) 1e+02))) (Variables|Default|GetLastSamplePosResult))
                      (bind _values (Utilities|Map|Values (Variables|Default|GetOnsetTimestampMap)))
                      (Variables|Default|SetSamplePosResult (Utilities|Array|Get(acopy) _values (+ (Utilities|Array|FindItem _values (Utilities|Array|Get(acopy) _nearestneighbourresults (Math|Float|Truncate (* (Variables|Default|GetScaledVelocity) 1e+02)))) (Math|Integer|SelectInt 1 -1 (Math|Random|RandomBool)))))
                      (else
                        (Variables|Default|SetSamplePosResult (Utilities|Array|Get(acopy) _nearestneighbourresults (Math|Float|Truncate (* (Variables|Default|GetScaledVelocity) 1e+02))))))))
                (:then_1
                  (Audio|Parameter|SetFloatParameter _audiocomponent "StartTime" (Variables|Default|GetSamplePosResult) :!class /Script/AudioExtensions.AudioParameterControllerInterface)
                  (Audio|Parameter|SetFloatParameter _audiocomponent "Velocity" (Variables|Default|GetScaledVelocity) :!class /Script/AudioExtensions.AudioParameterControllerInterface))))))))
    (:then_1
      (Utilities|FlowControl|Delay (Math|Random|RandomFloatinRange 0.3 0.5))
      (goto _label Reset))))

(event Custom|TriggerHitSounds
  (params (Velocity :type Vector) (NewTransform :type Transform%20%28by%20ref%29)))

(event EventBeginPlay
  (bind _owner (Variables|Default|GetOwner))
  (Private|Init)
  (if (Utilities|IsValid _owner)
    (Collision|BindEventtoOnActorHit _owner (delegate Custom|OnActorhit))))

(fn Init
  (bind _returnvalue (Components|GetOwner))
  (Variables|Default|SetIsInitialized true)
  (bind _output_get (Variables|Default|SetOwner _returnvalue))
  (bind _returnvalue_2 (Game|SpawnActorfromClass "/Script/Engine.AmbientSound" (Transformation|GetActorTransform _returnvalue) "Undefined" _output_get 0))
  (bind _output_get_2 (Variables|Default|SetAudioComponent (Variables|/Script/Engine.AmbientSound|GetAudioComponent _returnvalue_2)))
  (Audio|Components|Audio|SetSound _output_get_2 (Variables|Default|GetMetaSoundAsset))
  (Variables|/Script/Engine.AudioComponent|SetAttenuationSettings _output_get_2 (Variables|Default|GetAttenuation))
  (Variables|/Script/Engine.AudioComponent|SetConcurrencySet _output_get_2 (Variables|Default|GetConcurrency%20Set))
  (bind _returnvalue_3 (Actor|GetActorOfClass "/Game/Audio/BP/EUA_UpdateNRT.EUA_UpdateNRT_C"))
  (bind _aseua_update_nrt (Utilities|Casting|CastToEUA_UpdateNRT _returnvalue_3)
    (:then
      (bind _array_element (Utilities|Array|ForEachLoopwithBreak (Variables|/Game/Audio/BP/EUA_UpdateNRT.EUA_UpdateNRT_C|GetDT_OnsetNRT_Analysis _aseua_update_nrt) :!label _label)
        (:LoopBody
          (if (== (.name _array_element) (Variables|Public|GetSoundName))
            (Variables|Default|SetNearestNeighbourResults (.n100_onsetnrt_results_timing _array_element))
            (Variables|Default|SetOnsetTimestampMap (.onsetnrt_datamap _array_element))
            (bind _output_get_3 (Variables|Default|SetWaveAsset (.waveasset _array_element)))
            (Class|AudioComponent|SetWaveParameter (Variables|Default|GetAudioComponent) "WaveAsset" _output_get_3)
            (goto _label Break)))))
    (:CastFailed
      (Development|PrintString "bp bad"))))