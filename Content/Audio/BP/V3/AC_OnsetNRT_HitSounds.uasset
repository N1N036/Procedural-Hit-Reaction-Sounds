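; Actor component that plays velocity-matched impact sounds when its static mesh actor is hit.
; Init spawns an AmbientSound running a MetaSound and loads precomputed onset analysis from EUA_UpdateNRT, matched by sound name or surface type.
; Hits use scaled speed, with random jitter, to look up an onset timestamp through a nearest-neighbour table.
; The MetaSound receives that start time, velocity and a volume correction at the impact point, with randomly timed retrigger gating.
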(event Custom|OnActorhit
  (params (SelfActor :type Actor%20Object%20Reference) (OtherActor :type Actor%20Object%20Reference) (NormalImpulse :type Vector) (Hit :type Hit%20Result%20Structure%20%28by%20ref%29))
  (bind _returnvalue (Transformation|GetVelocity OtherActor))
  (bind _onsettimestampmap (Variables|Default|GetOnsetTimestampMap))
  (bind _audiocomponent (Variables|Default|GetAudioComponent))
  (bind _static_surface (Variables|Default|GetStatic%20Surface))
  (bind _nearestneighbourresults (Variables|Default|GetNearestNeighbourResults))
  (bind _owner (Variables|Default|GetOwner))
  (bind _returnvalue_2 (Transformation|GetVelocity _owner))
  (bind _returnvalue_3 (Math|Vector|SelectVector _returnvalue _returnvalue_2 _static_surface))
  (bind _returnvalue_4 (Math|Vector|VectorLength _returnvalue_3))
  (Utilities|FlowControl|Sequence
    (:then_0
      (Utilities|FlowControl|DoOnce false :!label _label
        (:Completed
          (if (not (Audio|Components|Audio|IsPlaying (Audio|Components|Audio|GetPlayState (Variables|Default|GetAudioComponent))))
            (if (> _returnvalue_4 1e+01)
              (Variables|Default|SetScaledVelocity (Math|Float|Clamp(Float) (/ _returnvalue_4 1e+03)))
              (Transformation|SetWorldTransform _audiocomponent (Math|Conversions|ToTransform(Vector) (.impactpoint Hit)) false true)
              (Audio|Components|Audio|Play _audiocomponent 0.0)
              (Utilities|FlowControl|Sequence
                (:then_0
                  (if (Utilities|Array|IsValidIndex _nearestneighbourresults (Math|Integer|Clamp(Integer) (+ (Math|Float|Truncate (* (Variables|Default|GetScaledVelocity) 1e+02)) (Math|Random|RandomIntegerinRange -2 2)) 0 100))
                    (bind _values (Utilities|Map|Values _onsettimestampmap))
                    (bind _keys (Utilities|Map|Keys _onsettimestampmap))
                    (Variables|Default|SetSamplePosResult (Utilities|Array|Get(acopy) _values (Math|Integer|Clamp(Integer) (+ (Utilities|Array|FindItem _values (Utilities|Array|Get(acopy) _nearestneighbourresults (Math|Integer|Clamp(Integer) (+ (Math|Float|Truncate (* (Variables|Default|GetScaledVelocity) 1e+02)) (Math|Random|RandomIntegerinRange -2 2)) 0 100))) (Math|Random|RandomIntegerinRange -2 2)) 0 (- (Utilities|Array|Length _values) 1))))
                    (Variables|Default|SetDeltaVolume (Math|Float|SafeDivide (Variables|Default|GetScaledVelocity) (Utilities|Array|Get(acopy) _keys (Math|Integer|Clamp(Integer) (+ (Utilities|Array|FindItem _values (Utilities|Array|Get(acopy) _nearestneighbourresults (Math|Integer|Clamp(Integer) (+ (Math|Float|Truncate (* (Variables|Default|GetScaledVelocity) 1e+02)) (Math|Random|RandomIntegerinRange -2 2)) 0 100))) (Math|Random|RandomIntegerinRange -2 2)) 0 (- (Utilities|Array|Length _values) 1)))))
                    (else
                      (Development|PrintString "No valid int bp baddddd" true true "(R=1.000000,G=0.031819,B=0.000000,A=1.000000)"))))
                (:then_1
                  (Audio|Parameter|SetFloatParameter (Variables|Default|GetAudioComponent) "StartTime" (Variables|Default|GetSamplePosResult) :!class /Script/AudioExtensions.AudioParameterControllerInterface)
                  (Audio|Parameter|SetFloatParameter (Variables|Default|GetAudioComponent) "Velocity" (Variables|Default|GetScaledVelocity) :!class /Script/AudioExtensions.AudioParameterControllerInterface)
                  (Audio|Parameter|SetFloatParameter (Variables|Default|GetAudioComponent) "DeltaVolume" (Variables|Default|GetDeltaVolume) :!class /Script/AudioExtensions.AudioParameterControllerInterface)
                  (if (Variables|Default|GetDebug)
                    (Development|PrintString (Utilities|String|Append (Utilities|String|ToString(Float) (Variables|Default|GetSamplePosResult)) "---" (Utilities|String|ToString(Float) (Variables|Default|GetScaledVelocity))))))))))))
    (:then_1
      (Utilities|FlowControl|Delay (Math|Random|RandomFloatinRange 0.01 0.2))
      (goto _label Reset))))

(event EventTick
  (params (DeltaSeconds :type Float%20%28single-precision%29))
  (Variables|Default|SetScaledVelocity (+ (Variables|Default|GetScaledVelocity) 0.01)))

(event EventBeginPlay
  (Class|ActorComponent|SetComponentTickInterval 0.5)
  (Components|Tick|SetComponentTickEnabled (Variables|Default|GetDebug))
  (bind _asstatic_mesh_actor (Private|Init))
  (Collision|BindEventtoOnActorHit _asstatic_mesh_actor (delegate Custom|OnActorhit)))

(fn Init
  (bind _returnvalue (Components|GetOwner))
  (bind _soundname (Variables|Public|GetSoundName))
  (Variables|Default|SetIsInitialized true)
  (if (Utilities|IsValid _returnvalue)
    (bind _output_get (Variables|Default|SetOwner _returnvalue))
    (bind _returnvalue_2 (Game|SpawnActorfromClass "/Script/Engine.AmbientSound" (Transformation|GetActorTransform _returnvalue) "Undefined" _output_get 0))
    (bind _output_get_2 (Variables|Default|SetAudioComponent (Variables|/Script/Engine.AmbientSound|GetAudioComponent _returnvalue_2)))
    (Audio|Components|Audio|SetSound _output_get_2 (Variables|Default|GetMetaSoundAsset))
    (Variables|/Script/Engine.AudioComponent|SetAttenuationSettings _output_get_2 (Variables|Default|GetAttenuation))
    (Variables|/Script/Engine.AudioComponent|SetConcurrencySet _output_get_2 (Variables|Default|GetConcurrency%20Set))
    (bind _asstatic_mesh_actor (Utilities|Casting|CastToStaticMeshActor (Variables|Default|GetOwner)))
    (Variables|Default|SetStatic%20Surface (not (Physics|IsSimulatingPhysics (Variables|/Script/Engine.StaticMeshActor|GetStaticMeshComponent _asstatic_mesh_actor) "None")))
    (bind _returnvalue_3 (Actor|GetActorOfClass "/Game/Audio/BP/V3/EUA_UpdateNRT.EUA_UpdateNRT_C"))
    (bind _aseua_update_nrt (Utilities|Casting|CastToEUA_UpdateNRT _returnvalue_3)
      (:then
        (LocalVariables|SetSurface%20Type (Variables|/Script/PhysicsCore.PhysicalMaterial|GetSurfaceType (Class|MaterialInterface|GetPhysicalMaterial (Rendering|Material|GetMaterial (Variables|/Script/Engine.StaticMeshActor|GetStaticMeshComponent _asstatic_mesh_actor) 0))))
        (bind _array_element (Utilities|Array|ForEachLoopwithBreak (Variables|/Game/Audio/BP/V3/EUA_UpdateNRT.EUA_UpdateNRT_C|GetDT_OnsetNRT_Analysis _aseua_update_nrt) :!label _label)
          (:LoopBody
            (if (and (== (.name _array_element) _soundname) (!= _soundname "None"))
              (Variables|Default|SetNearestNeighbourResults (.n100_onsetnrt_results_timing _array_element) :!label _label_2)
              (Development|PrintString "Hello")
              (Variables|Default|SetOnsetTimestampMap (.onsetnrt_datamap _array_element))
              (bind _output_get_3 (Variables|Default|SetWaveAsset (.waveasset _array_element)))
              (Class|AudioComponent|SetWaveParameter (Variables|Default|GetAudioComponent) "WaveAsset" _output_get_3)
              (goto _label Break)
              (elif (and (Utilities|Enum|Equal(Enum) (.physical_material _array_element) (LocalVariables|GetSurface%20Type)) (Utilities|Enum|NotEqual(Enum) (LocalVariables|GetSurface%20Type) "SurfaceType_Default"))
                (goto _label_2))))
          (:Completed
            (return _asstatic_mesh_actor))))
      (:CastFailed
        (Development|PrintString "bp bad" true true "(R=1.000000,G=0.019947,B=0.059748,A=1.000000)")))))