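; Actor component for procedural impact sounds that plays a MetaSound on a new audio component when its owner is hit.
; BeginPlay also maps audio onset strengths to timestamps from an onset analysis asset.
; Hits pass a speed check and random cooldown, then compute a jittered, normalized velocity before playback.
; Disconnected logic would randomize modal synthesis arrays or pick the onset nearest that velocity, so live playback receives no parameters.
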(event EventTick
  (params (DeltaSeconds :type Float%20%28single-precision%29)))

(event Custom|trigger
  (params (SelfActor :type Actor%20Object%20Reference) (OtherActor :type Actor%20Object%20Reference) (NormalImpulse :type Vector) (Hit :type Hit%20Result%20Structure%20%28by%20ref%29))
  (CallFunction|TriggerHitSounds)
  (Development|PrintString "hit"))

(event EventBeginPlay
  (bind _returnvalue (Components|GetOwner))
  (Collision|BindEventtoOnActorHit _returnvalue (delegate Custom|trigger))
  (CallFunction|StartOnsetAnalasys)
  (bind _returnvalue_2 (Game|AddComponentbyClass _returnvalue "/Script/Engine.AudioComponent" false))
  (bind _output_get (Variables|Default|SetSoundActor _returnvalue_2))
  (Audio|Components|Audio|SetSound _output_get (Variables|Default|GetMSS_TransientSelect)))

(event Custom|TriggerHitSounds
  (bind _returnvalue (Components|GetOwner))
  (bind _returnvalue_2 (Transformation|GetVelocity _returnvalue))
  (bind _returnvalue_3 (Math|Vector|VectorLength _returnvalue_2))
  (Utilities|FlowControl|Sequence
    (:then_0
      (Utilities|FlowControl|Sequence
        (:then_0
          (Utilities|FlowControl|DoOnce false :!label _label
            (:Completed
              (if (> _returnvalue_3 0.1)
                (Variables|Default|SetScaledVelocity (- (Math|Float|Clamp(Float) (Math|Float|SafeDivide _returnvalue_3 3e+03)) (Math|Random|RandomFloatinRange 0.0 0.1)))
                (Audio|Components|Audio|Play (Variables|Default|GetSoundActor) 0.0)))))
        (:then_1
          (Utilities|FlowControl|Delay (Math|Random|RandomFloatinRange 0.4 2.0))
          (goto _label Reset))))
    (:then_1
      (if (Variables|Default|GetDebug)
        (Class|VisualLoggerKismetLibrary|LogLocation (Variables|Default|GetSoundActor) "0, 0, 0" "Bonk" "(R=0.000000,G=0.000000,B=1.000000,A=1.000000)" 1e+01 "VisLogBP")))))

(event Custom|StartOnsetAnalasys
  (bind _target (Variables|Default|GetTarget))
  (bind _durationinseconds (Variables|/Script/AudioAnalyzer.AudioAnalyzerNRT|GetDurationInSeconds _target))
  (bind (_outonsettimestamps _outonsetstrengths) (Class|OnsetNRT|GetNormalizedChannelOnsetsBetweenTimes _target 0.0 _durationinseconds))
  (for (_array_element _array_index) _outonsettimestamps
    (Utilities|Map|Add (Variables|Default|GetOnsetTimestampMap) (Utilities|Array|Get(acopy) _outonsetstrengths _array_index) _array_element)))